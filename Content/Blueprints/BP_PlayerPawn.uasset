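; BP_PlayerPawn is a player pawn that moves and turns itself on Tick, with no movement component calls in its graph.
; Each frame it consumes the pending movement input, scales it by MovementSpeed and delta time, and applies it as a swept world offset.
; Non-zero movement updates DesiredRotation, and the pawn continually lerps toward it along the shortest path at a rate set by RotationSpeed.
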(event Collision|EventActorBeginOverlap
  (params (OtherActor :type Actor%20Object%20Reference)))

(event EventTick
  (params (DeltaSeconds :type Float%20%28single-precision%29))
  ;[1 1 1] Movement
  (bind _returnvalue (Class|Pawn|ConsumeMovementInputVector))
  (Transformation|AddActorWorldOffset (* (* _returnvalue DeltaSeconds) (Variables|PawnMovement|GetMovementSpeed)) true)
  ;[1 1 1] Calculate desired rotation
  ;;[1 1 1] Is there movement input detected?
  (if (> (Math|Vector|VectorLengthSquared (* (* _returnvalue DeltaSeconds) (Variables|PawnMovement|GetMovementSpeed))) 0.0)
    (Variables|PawnMovement|SetDesiredRotation (Math|Conversions|RotationFromXVector (* (* _returnvalue DeltaSeconds) (Variables|PawnMovement|GetMovementSpeed)))))
  ;[1 0.1237 0.5589] Rotate pawn to DesiredRotation
  (Transformation|SetActorRotation (Math|Rotator|Lerp(Rotator) (Transformation|GetActorRotation) (Variables|PawnMovement|GetDesiredRotation) (* DeltaSeconds (Variables|PawnMovement|GetRotationSpeed)) true)))

(fn ConstructionScript)