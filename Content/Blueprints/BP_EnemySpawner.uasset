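; Enemy spawner that replaces the current enemy with the one for the player's current round.
; Spawn destroys actors tagged "Enemy", then spawns an AI from a five-class array indexed by the player controller's Round stat at a fixed location.
; It stores that location, exposed through a getter, and the original material of the first BP_EnemyCharacter found.
; A hit event briefly swaps that material to flash the enemy as damage feedback.
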(event Custom|Spawn
  ;[1 1 1] Delete old enemy and spawn new one
  (bind _outactors (Actor|GetAllActorswithTag "Enemy"))
  (Actor|DestroyActor _outactors)
  (bind _asbp_my_player_controller (Utilities|Casting|CastToBP_MyPlayerController (Game|GetPlayerController 0)))
  (bind _returnvalue (AI|SpawnAIFromClass (Utilities|Array|Get(acopy) (Variables|Default|GetEnemies) (Variables|/Game/Blueprints/BPC_Stats.BPC_Stats_C|GetRound (Variables|/Game/Blueprints/BP_MyPlayerController.BP_MyPlayerController_C|GetBPC_Stats _asbp_my_player_controller))) 0 "250.000000,0.000000,140.000000" "0.000000,180.000000,0.000000" false 0))
  (Variables|Default|SetEnemySpawnLocation (Transformation|GetActorLocation _returnvalue))
  (bind _outactors_2 (Actor|GetAllActorsOfClass "/Game/Blueprints/BP_EnemyCharacter.BP_EnemyCharacter_C"))
  (Variables|Default|SetStartMaterial (Rendering|Material|GetMaterial (Variables|/Script/Engine.Character|GetMesh (Utilities|Array|Get(acopy) _outactors_2)) 0)))

(event Custom|EnemyHitBodyColorIndicator
  ;[1 1 1] Color indicator when player hits enemy
  (bind _outactors (Actor|GetAllActorsOfClass "/Game/Blueprints/BP_EnemyCharacter.BP_EnemyCharacter_C"))
  (Rendering|Material|SetMaterial (Variables|/Script/Engine.Character|GetMesh (Utilities|Array|Get(acopy) _outactors)) 0 "/Game/Materials/M_BaseProjectile.M_BaseProjectile")
  (Utilities|FlowControl|Delay 0.25)
  (Rendering|Material|SetMaterial (Variables|/Script/Engine.Character|GetMesh (Utilities|Array|Get(acopy) _outactors)) 0 (Variables|Default|GetStartMaterial)))

(event EventBeginPlay
  (Variables|Default|SetEnemies (Utilities|Array|MakeArray "/Game/Blueprints/BP_EnemyCharacter.BP_EnemyCharacter_C" "/Game/Blueprints/BP_EnemyCharacter2.BP_EnemyCharacter2_C" "/Game/Blueprints/BP_EnemyCharacter3.BP_EnemyCharacter3_C" "/Game/Blueprints/BP_EnemyCharacter4.BP_EnemyCharacter4_C" "/Game/Blueprints/BP_EnemyCharacter5.BP_EnemyCharacter5_C")))

(event Collision|EventActorBeginOverlap
  (params (OtherActor :type Actor%20Object%20Reference)))

(event EventTick
  (params (DeltaSeconds :type Float%20%28single-precision%29)))

(fn ConstructionScript)

(fn GetEnemySpawnLocation
  (return (Variables|Default|GetEnemySpawnLocation)))