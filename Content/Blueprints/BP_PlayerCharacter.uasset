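; BP_PlayerCharacter is the player character Blueprint, handling spawn placement and death.
; On BeginPlay it moves itself to a fixed location 150 units above the world origin.
; When its BPC_Health component fires OnDeath, it tells BP_MyPlayerController the round is over, asks BP_MyGameMode to respawn the player, then destroys itself.
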(event OnDeath(BPC_Health)
  (bind _asbp_my_player_controller (Utilities|Casting|CastToBP_MyPlayerController (Game|GetPlayerController 0)))
  (Default|RoundOver _asbp_my_player_controller)
  (bind _asbp_my_game_mode (Utilities|Casting|CastToBP_MyGameMode (Game|GetGameMode))
    (:then
      (Default|RespawnPlayer _asbp_my_game_mode))
    (:CastFailed
      _))
  (Actor|DestroyActor self))

(event EventBeginPlay
  (|CallParentFunction)
  (Transformation|SetActorTransform (Math|Transform|MakeTransform "0.000000,0.000000,150.000000" "0, 0, 0" "1.000000,1.000000,1.000000")))

(event Collision|EventActorBeginOverlap
  (params (OtherActor :type Actor%20Object%20Reference))
  (|CallParentFunction OtherActor) ; This node is disabled and will not be called.\nDrag off pins to build functionality.
)

(event EventTick
  (params (DeltaSeconds :type Float%20%28single-precision%29))
  (|CallParentFunction DeltaSeconds))

(fn ConstructionScript
  (|CallParentFunction))