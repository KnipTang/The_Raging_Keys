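; Stats component that tracks points, round and combo for a round-based game with combo key prompts.
; Events increment points and round, while combo changes are clamped at zero and trigger enemy increase or decrease animations on the game HUD.
; A next-round event scales difficulty by raising the combo actor's max key speed and shortening the player controller timer's max time down to a fixed floor.
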(event Custom|IncreaseRound
  (bind _result (Math|Integer|IncrementInt (Variables|Default|GetRound))
    (:%20%20
      (Variables|Default|SetRound _result))))

(event Custom|IncreasePoints
  (bind _result (Math|Integer|IncrementInt (Variables|Default|GetPoints))
    (:%20%20
      (Variables|Default|SetPoints _result))))

(event Custom|IncreaseCombo
  (params (Amount :type Float%20%28double-precision%29))
  ;[1 1 1] Increase/Decrease enemies health
  (if (<= (+ Amount (Variables|Default|GetCombo)) 0.0)
    (Variables|Default|SetCombo 0.0)
    (else
      (Variables|Default|SetCombo (+ Amount (Variables|Default|GetCombo)))))
  (if (<= Amount 0.0)
    (bind _foundwidgets (Widget|GetAllWidgetsOfClass "/Game/Blueprints/BPW_GameHud.BPW_GameHud_C" true))
    (Default|PlayEnemyIncreaseAnimation _foundwidgets)
    (else
      (bind _foundwidgets_2 (Widget|GetAllWidgetsOfClass "/Game/Blueprints/BPW_GameHud.BPW_GameHud_C" true))
      (Default|PlayEnemyDecreaseAnimation _foundwidgets_2))))

(event Custom|NextRoundUpdateStats
  ;[1 1 1] Update stats when new rounds starts
  (bind _asbp_my_player_controller (Utilities|Casting|CastToBP_MyPlayerController (Game|GetPlayerController 0)))
  (bind _returnvalue (Actor|GetActorOfClass "/Game/Blueprints/BP_Combo.BP_Combo_C"))
  (Default|SetKeyMaxSpeed _returnvalue (+ (Variables|/Game/Blueprints/BP_Combo.BP_Combo_C|GetMaxKeySpeed _returnvalue) 1e+02))
  (if (< (- (Variables|/Game/Blueprints/BPC_Timer.BPC_Timer_C|GetMaxTime (Variables|/Game/Blueprints/BP_MyPlayerController.BP_MyPlayerController_C|GetBPC_Timer _asbp_my_player_controller)) 0.5) 0.5)
    (Default|SetMaxTime (Variables|/Game/Blueprints/BP_MyPlayerController.BP_MyPlayerController_C|GetBPC_Timer _asbp_my_player_controller) 0.5)
    (else
      (Default|SetMaxTime (Variables|/Game/Blueprints/BP_MyPlayerController.BP_MyPlayerController_C|GetBPC_Timer _asbp_my_player_controller) (- (Variables|/Game/Blueprints/BPC_Timer.BPC_Timer_C|GetMaxTime (Variables|/Game/Blueprints/BP_MyPlayerController.BP_MyPlayerController_C|GetBPC_Timer _asbp_my_player_controller)) 0.5)))))

(event EventBeginPlay)

(event EventTick
  (params (DeltaSeconds :type Float%20%28single-precision%29)))