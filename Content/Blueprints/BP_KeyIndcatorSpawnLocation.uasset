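; BP_KeyIndcatorSpawnLocation is a helper Blueprint that picks randomized 2D spawn positions for key indicators.
; GetLocation offsets the BP_EnemySpawner's enemy spawn location by a random left or right X and a random Y.
; GetComboKeyLocation returns a random X on a fixed Y, independent of the spawner.
; Both functions also set a LeftSide flag from the chosen X, and the event graph is empty.
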(event EventBeginPlay)

(event Collision|EventActorBeginOverlap
  (params (OtherActor :type Actor%20Object%20Reference)))

(event EventTick
  (params (DeltaSeconds :type Float%20%28single-precision%29)))

(fn ConstructionScript)

(fn GetLocation
  (LocalVariables|SetYvalue (Math|Random|RandomFloatinRange 0.0 5e+02))
  (if (Math|Random|RandomBool)
    (LocalVariables|SetXvalue -5e+01)
    (Variables|Default|SetLeftSide false)
    (else
      (LocalVariables|SetXvalue -5e+02)
      (Variables|Default|SetLeftSide true)))
  (bind _returnvalue (Actor|GetActorOfClass "/Game/Blueprints/BP_EnemySpawner.BP_EnemySpawner_C"))
  (bind _enemyspawnlocation (Default|GetEnemySpawnLocation _returnvalue))
  (return (Math|Vector2D|MakeVector2D (+ (.x _enemyspawnlocation) (LocalVariables|GetXvalue)) (+ (.y _enemyspawnlocation) (LocalVariables|GetYvalue)))))

(fn GetComboKeyLocation
  (LocalVariables|SetYvalue -2e+02)
  (bind _output_get (LocalVariables|SetXvalue (Math|Random|RandomFloatinRange -9e+02 7e+02)))
  (if (<= _output_get -8e+02)
    (Variables|Default|SetLeftSide true)
    (else
      (Variables|Default|SetLeftSide false)))
  (return (Math|Vector2D|MakeVector2D (LocalVariables|GetXvalue) (LocalVariables|GetYvalue))))