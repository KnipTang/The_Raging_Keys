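; BPC_Rage is a Blueprint component that tracks a rage meter for its owner.
; The IncreaseRage event adds a fixed amount to CurrentRage without clamping it to MaxRage.
; Helper functions return the current-to-max ratio, report whether rage has reached the maximum, and reset it to a small non-zero value.
; BeginPlay and Tick are unused, so rage changes only when IncreaseRage or ResetRage is called.
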(event Custom|Increase%20Rage
  (Variables|Default|SetCurrent%20Rage (+ (Variables|Default|GetCurrent%20Rage) 1e+01)))

(event EventBeginPlay)

(event EventTick
  (params (DeltaSeconds :type Float%20%28single-precision%29)))

(fn GEtRagePercentage
  (return (/ (Variables|Default|GetCurrent%20Rage) (Variables|Default|GetMax%20Rage))))

(fn IsRageMax
  (return (>= (Variables|Default|GetCurrent%20Rage) (Variables|Default|GetMax%20Rage))))

(fn ResetRage
  (Variables|Default|SetCurrent%20Rage 0.1))