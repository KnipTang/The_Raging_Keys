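; BPC_Timer is a round timer component that counts up to a maximum time and notifies the player controller when time runs out.
; While the round is started, Tick accumulates delta time and calls TimeRunsOut on BP_MyPlayerController every frame at or past the limit, without stopping or resetting itself.
; Events start, stop and reset the timer, while functions set the maximum and return elapsed time as a fraction.
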(event Custom|Stop%20Timer
  (Variables|Default|SetRoundStarted false))

(event Custom|ResetCurrentTime
  (Variables|Default|SetCurrentTime 0.0))

(event Custom|Start%20timer
  (Variables|Default|SetRoundStarted true))

(event EventBeginPlay)

(event EventTick
  (params (DeltaSeconds :type Float%20%28single-precision%29))
  ;[1 1 1] Check if round has been started
  (if (Variables|Default|GetRoundStarted)
    ;[1 1 1] Increase Timer
    (bind _output_get (Variables|Default|SetCurrentTime (+ DeltaSeconds (Variables|Default|GetCurrentTime))))
    ;[1 1 1] Check if time hit max
    (if (>= _output_get (Variables|Default|GetMaxTime))
      ;[1 1 1] Damage if time runs out
      (bind _asbp_my_player_controller (Utilities|Casting|CastToBP_MyPlayerController (Game|GetPlayerController 0)))
      (Default|TimeRunsOut _asbp_my_player_controller))))

(fn SetMaxTime
  (params (NewMaxTime :type Float%20%28double-precision%29))
  (Variables|Default|SetMaxTime NewMaxTime))

(fn GetTimerPercentage
  (return (/ (Variables|Default|GetCurrentTime) (Variables|Default|GetMaxTime))))