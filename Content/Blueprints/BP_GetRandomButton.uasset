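; BP_GetRandomButton picks a random letter as the current button, based on the player's round.
; It runs GetRandomLetter on BeginPlay and whenever GetButtonEvent is called.
; That function reads Round from the BPCStats of BP_MyPlayerController and passes it to the GetRandomKey2 actor found in the level.
; The result is stored in RandomButton and returned.
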(event Custom|GetButtonEvent
  (CallFunction|GetRandomLetter))

(event EventBeginPlay
  (CallFunction|GetRandomLetter))

(event Collision|EventActorBeginOverlap
  (params (OtherActor :type Actor%20Object%20Reference)))

(event EventTick
  (params (DeltaSeconds :type Float%20%28single-precision%29)))

(fn ConstructionScript)

(fn GetRandomLetter
  (bind _asbp_my_player_controller (Utilities|Casting|CastToBP_MyPlayerController (Game|GetPlayerController 0)))
  (bind _returnvalue (Actor|GetActorOfClass "/Script/Unreal101.GetRandomKey2"))
  (bind _output_get (Variables|Default|SetRandomButton (Class|GetRandomKey2|GetRandomLetter _returnvalue (Variables|/Game/Blueprints/BPC_Stats.BPC_Stats_C|GetRound (Variables|/Game/Blueprints/BP_MyPlayerController.BP_MyPlayerController_C|GetBPC_Stats _asbp_my_player_controller)))))
  (return _output_get))